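; Player controller that turns Enhanced Input into movement, aiming, interaction and camera zoom for a referenced player character.
; Movement follows control yaw, and holding left click switches off orient-to-movement and turns the character toward the mouse cursor position.
; Interact messages the character's look-at actor and broadcasts the returned value as an objective ID.
; Scroll adjusts spring arm length within clamped limits, and the character reference is supplied through SetPlayerREF.
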(event `self.ReceiveBeginPlay`
  (bind _returnvalue (pcsubsystem `EnhancedInputLocalPlayerSubsystem` self))
  (`/Engine/EditorBlueprintResources/StandardMacros.IsValid` _returnvalue
    (:`Is Valid`
      (`EnhancedInputSubsystemInterface.AddMappingContext` _returnvalue "/Game/Framework/Controller/IMC_General.IMC_General" 0 (struct)))
    (:`Is Not Valid`
      (`KismetSystemLibrary.PrintString` "Enhanced Input system was not valid - BP_PlayerController::BegintPlay()"))))

(event `EnhancedInput|/Game/Framework/Controller/IA_Move`
  (params (ActionValue :type "Vector2D Structure") (ElapsedSeconds :type "Float (double-precision)") (TriggeredSeconds :type "Float (double-precision)") (InputAction :type "InputAction Object Reference" :default "/Game/Framework/Controller/IA_Move.IA_Move"))
  (bind (_returnvalue_roll _returnvalue_pitch _returnvalue_yaw) (`KismetMathLibrary.BreakRotator` (`self.GetControlRotation`)))
  (bind (_returnvalue_roll_2 _returnvalue_pitch_2 _returnvalue_yaw_2) (`KismetMathLibrary.BreakRotator` (`self.GetControlRotation`)))
  (:`Triggered`
    (`Pawn.AddMovementInput` (`self.Playe_REF`) (`KismetMathLibrary.GetForwardVector` (`KismetMathLibrary.MakeRotator` 0.0 0.0 _returnvalue_yaw)) ActionValue_X false)
    (`Pawn.AddMovementInput` (`self.Playe_REF`) (`KismetMathLibrary.GetRightVector` (`KismetMathLibrary.MakeRotator` _returnvalue_roll_2 0.0 _returnvalue_yaw_2)) ActionValue_Y false)))

(event `EnhancedInput|/Game/Framework/Controller/IA_LeftClick`
  (params (ActionValue :type Boolean) (ElapsedSeconds :type "Float (double-precision)") (TriggeredSeconds :type "Float (double-precision)") (InputAction :type "InputAction Object Reference" :default "/Game/Framework/Controller/IA_LeftClick.IA_LeftClick"))
  (bind _playe_ref (`self.Playe_REF`))
  (bind _charactermovement (`Character.CharacterMovement` (`self.Playe_REF`)))
  (bind (_returnvalue_roll _returnvalue_pitch _returnvalue_yaw) (`KismetMathLibrary.BreakRotator` (`KismetMathLibrary.MakeRotFromX` (- (`self.MouseCursor`) (`self.K2_GetActorLocation` _playe_ref)))))
  (:`Triggered`
    (set `CharacterMovementComponent.bOrientRotationToMovement` false _charactermovement)
    (`self.K2_SetActorRotation` _playe_ref (`KismetMathLibrary.MakeRotator` 0.0 0.0 _returnvalue_yaw) false))
  (:`Completed`
    (set `CharacterMovementComponent.bOrientRotationToMovement` true _charactermovement)))

(event `EnhancedInput|/Game/Framework/Controller/IA_Interact`
  (params (ActionValue :type Boolean) (ElapsedSeconds :type "Float (double-precision)") (TriggeredSeconds :type "Float (double-precision)") (InputAction :type "InputAction Object Reference" :default "/Game/Framework/Controller/IA_Interact.IA_Interact"))
  ; Change this to work with "Left_Click"
  (:`Started`
    (bind _objectiveid (message `/Game/Framework/NPC/InteractionInterface.InteractWith` (`/Game/Framework/BP_PlayableCharacter.LookAtActor` (`self.Playe_REF`))))
    (`self.OnObjectiveIDCalled` _objectiveid)))

(event `EnhancedInput|/Game/Framework/Controller/IA_CameraScroll`
  (params (ActionValue :type "Float (double-precision)") (ElapsedSeconds :type "Float (double-precision)") (TriggeredSeconds :type "Float (double-precision)") (InputAction :type "InputAction Object Reference" :default "/Game/Framework/Controller/IA_CameraScroll.IA_CameraScroll"))
  (bind _springarm (`/Game/Framework/BP_PlayableCharacter.SpringArm` (`self.Playe_REF`)))
  ; Clean this
  (:`Started`
    (set `SpringArmComponent.TargetArmLength` (`KismetMathLibrary.FClamp` (+ (`SpringArmComponent.TargetArmLength` _springarm) (* ActionValue 100.0)) 300.0 2000.0) _springarm)))

(fn `SetPlayerREF`
  (params (InPlayer_REF :type "/Game/Framework/BP_PlayableCharacter Object Reference"))
  (set `self.Playe_REF` InPlayer_REF))

(fn `UserConstructionScript`)