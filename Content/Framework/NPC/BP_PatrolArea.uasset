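; BP_PatrolArea is a spline-outlined area for NPC patrols that supplies random locations inside its boundary.
; The construction script calls SetAllPointsLinear to give the spline straight edges.
; FindRandLocation repeatedly picks two random spline points and interpolates between them until IsPointInTriangle accepts the result.
; TestArea is a debug tool that spawns TEST actors at many sampled locations to check the boundaries.
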(event `self.ReceiveBeginPlay`)

(fn `FindRandLocation`
  (returns (NewLocation :type "Vector Structure"))
  (locals (bValidLocation :type Boolean))
  (while (not (`local.bValidLocation`))
    (set `self.Point_A` (`self.GetRandPointOnSpline`))
    (set `self.Point_B` (`self.GetRandPointOnSpline`))
    (bind _output_get (set `self.tempLocation` (`self.LERP`)))
    (bind _returnvalue (`self.isPointInTriangle` _output_get))
    (set `local.bValidLocation` _returnvalue))
  (return (`self.tempLocation`)))

(fn `TestArea`
  ; Debug tool to test boundaries
  (for _ (range 1001)
    (bind _newlocation (`self.FindRandLocation`))
    (`|SpawnActorFromClass` "/Game/Framework/NPC/Enemy/TEST.TEST_C" (`KismetMathLibrary.Conv_VectorToTransform` _newlocation) "Undefined" "MultiplyWithRoot" null null)))

(fn `UserConstructionScript`
  (`self.SetAllPointsLinear`))