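; Playable character Blueprint that sets up starting combat abilities and gives cursor feedback over interactable objects.
; On BeginPlay it adds sword slash and shield block abilities to indexed slots on its ability system component, if that component is valid.
; Every Tick it line traces from the deprojected mouse position on the Camera channel, switching the cursor to crosshairs when the hit actor implements the Interactable interface, otherwise default.
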(event `self.ReceiveBeginPlay`
  (bind _abilitysystemcomponent (`self.AbilitySystemComponent`))
  (`/Engine/EditorBlueprintResources/StandardMacros.IsValid` _abilitysystemcomponent
    (:`Is Valid`
      (`AbilitySystem.AddAbility` _abilitysystemcomponent "/Script/Project_D.SwordSlash" 0)
      (`AbilitySystem.AddAbility` _abilitysystemcomponent "/Script/Project_D.ShieldBlock" 1))))

(event `self.ReceiveTick`
  (params (DeltaSeconds :type "Float (single-precision)"))
  (bind _returnvalue (`GameplayStatics.GetPlayerController` 0))
  (bind (_worldlocation _worlddirection) (`PlayerController.DeprojectMousePositionToWorld` (`GameplayStatics.GetPlayerController` 0)))
  (bind _outhit (`KismetSystemLibrary.LineTraceSingle` _worldlocation (+ _worldlocation (* _worlddirection 10000.0)) "TraceTypeQuery2"))
  (if (`KismetSystemLibrary.DoesImplementInterface` (`.HitActor` (`GameplayStatics.BreakHitResult` _outhit)) "/Game/Framework/Interafaces/Interactable.Interactable_C")
    (set `PlayerController.CurrentMouseCursor` "Crosshairs" _returnvalue)
    (else
      (set `PlayerController.CurrentMouseCursor` "Default" _returnvalue))))

(fn `UserConstructionScript`)