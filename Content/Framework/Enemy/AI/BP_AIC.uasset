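; Base AI controller for enemies that runs the BT_EnemyBase behavior tree on BeginPlay.
; AI Perception updates feed HandleSightSense, which responds only to sight stimuli from the first player character.
; It writes the player to the TargetActor blackboard key while seen, and on losing sight clears that key and stores the stimulus location as LastKnownLocation.
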(event `self.ReceiveBeginPlay`
  (`self.RunBehaviorTree` "/Game/Framework/Enemy/AI/BT_EnemyBase.BT_EnemyBase"))

(event `self.AIPerception.OnTargetPerceptionUpdated`
  (params (Actor :type "Actor Object Reference") (Stimulus :type "AIStimulus Structure"))
  (`self.HandleSightSense` Actor Stimulus))

(fn `HandleSightSense`
  (params (Actor :type "Actor Object Reference") (Stimulus :type "AIStimulus Structure"))
  (bind (_stimulus_age _stimulus_expirationage _stimulus_strength _stimulus_stimuluslocation) (break `AIStimulus` (`local.Stimulus`)))
  (bind (_stimulus_age_2 _stimulus_expirationage_2 _stimulus_strength_2 _stimulus_stimuluslocation_2 _stimulus_receiverlocation _stimulus_tag _stimulus_bsuccessfullysensed) (break `AIStimulus` (`local.Stimulus`)))
  (bind _returnvalue (`AIPerceptionSystem.GetSenseClassForStimulus` Stimulus))
  (if (and (== _returnvalue "/Script/AIModule.AISense_Sight") (== (`local.Actor`) (`GameplayStatics.GetPlayerCharacter` 0)))
    (`BlackboardComponent.SetValueAsObject` (`self.Blackboard`) "TargetActor" (`KismetMathLibrary.SelectObject` (`local.Actor`) null _stimulus_bsuccessfullysensed))
    (if (not _stimulus_bsuccessfullysensed)
      (`BlackboardComponent.SetValueAsVector` (`self.Blackboard`) "LastKnownLocation" _stimulus_stimuluslocation))
    (else
      (return))))

(fn `UserConstructionScript`)